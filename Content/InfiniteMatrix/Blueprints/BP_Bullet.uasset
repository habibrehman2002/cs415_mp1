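; BP_Bullet is a projectile actor that destroys enemies and awards score to the player.
; Each tick it sweeps forward along world X at twice the player's ForwardSpeed, scaled by delta time.
; On hit, it destroys any SM_Enemy it struck, calls IncreaseScore on the player, then destroys itself.
; It enables sphere collision on BeginPlay and expires after a short lifespan if nothing is hit.
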(event `self.ReceiveBeginPlay`
  (`self.SetLifeSpan` 5.0)
  (`PrimitiveComponent.SetCollisionEnabled` (`self.Sphere`) "QueryAndPhysics"))

(event `self.ReceiveTick`
  (params (DeltaSeconds :type "Float (single-precision)"))
  (`self.K2_AddActorWorldOffset` (`KismetMathLibrary.MakeVector` (* DeltaSeconds (`/Game/InfiniteMatrix/Blueprints/BP_Player.ForwardSpeed` (`self.Player`)) 2.0)) true))

(event `self.ReceiveHit`
  (params (MyComp :type "PrimitiveComponent Object Reference") (Other :type "Actor Object Reference") (OtherComp :type "PrimitiveComponent Object Reference") (bSelfMoved :type Boolean) (HitLocation :type "Vector Structure") (HitNormal :type "Vector Structure") (NormalImpulse :type "Vector Structure") (Hit :type "HitResult Structure (by ref)"))
  (bind _assm_enemy (cast `/Game/InfiniteMatrix/Blueprints/SM_Enemy` Other)
    (:`then`
      (`self.K2_DestroyActor` _assm_enemy)
      (`/Game/InfiniteMatrix/Blueprints/BP_Player.IncreaseScore` (`self.Player`)))
    (:`CastFailed`
      _))
  (`self.K2_DestroyActor`))

(fn `UserConstructionScript`)