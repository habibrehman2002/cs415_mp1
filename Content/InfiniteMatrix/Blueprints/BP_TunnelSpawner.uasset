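; Spawner actor that builds a chain of BP_Tunnel segments, each with a randomized wall and either an enemy or, rarely, a health pack at a random offset.
; On BeginPlay it clears existing tunnels, then lays three starting segments from the player's location, destroying all enemies after each spawn.
; Each new segment attaches at the newest one's SpawnPoint and receives a spawner reference, with SpawnTunnelAtSpawnPoint extending the chain.
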(event `self.ReceiveBeginPlay`
  (`self.SpawnInitialTunnels`))

(fn `Spawn Tunnel`
  (params (SpawnLocation :type "Vector Structure"))
  (bind _returnvalue (`KismetMathLibrary.RandomFloatInRange` 0.0 360.0))
  (bind _returnvalue_2 (`KismetMathLibrary.RandomFloatInRange` 0.0 360.0))
  (bind _returnvalue_3 (* _returnvalue (`KismetMathLibrary.DegSin` _returnvalue_2)))
  (bind _returnvalue_4 (* _returnvalue (`KismetMathLibrary.DegCos` _returnvalue_2)))
  (bind _returnvalue_5 (`|SpawnActorFromClass` "/Game/InfiniteMatrix/Blueprints/BP_Tunnel.BP_Tunnel_C" (`KismetMathLibrary.MakeTransform` SpawnLocation) "Undefined" "OverrideRootScale" null null))
  (bind _output_get (set `self.Newest Tunnel` _returnvalue_5))
  (set `/Game/InfiniteMatrix/Blueprints/BP_Tunnel.TunnelSpawner` self _output_get)
  (`/Game/InfiniteMatrix/Blueprints/BP_Tunnel.RandomizeWall` _output_get)
  (`/Engine/EditorBlueprintResources/StandardMacros.CompareInt` (`KismetMathLibrary.RandomInteger` 10)
    (:`>`
      (bind _returnvalue_6 (`|SpawnActorFromClass` "/Game/InfiniteMatrix/Blueprints/SM_Enemy.SM_Enemy_C" (`KismetMathLibrary.MakeTransform` SpawnLocation) "Undefined" "OverrideRootScale" null null))
      (`self.K2_AddActorLocalOffset` _returnvalue_6 (`KismetMathLibrary.MakeVector` (`KismetMathLibrary.RandomFloatInRange` 1300.0 2300.0) _returnvalue_4 _returnvalue_3) false false))
    (:`==`
      (bind _returnvalue_7 (`|SpawnActorFromClass` "/Game/InfiniteMatrix/Blueprints/SM_HealthPack.SM_HealthPack_C" (`KismetMathLibrary.MakeTransform` SpawnLocation) "Undefined" "OverrideRootScale" null null))
      (`self.K2_AddActorLocalOffset` _returnvalue_7 (`KismetMathLibrary.MakeVector` (`KismetMathLibrary.RandomFloatInRange` 750.0 2200.0) _returnvalue_4 _returnvalue_3) false false))))

(fn `SpawnInitialTunnels`
  (`|ExecutionSequence`
    (:`then_0`
      (bind _outactors (`GameplayStatics.GetAllActorsOfClass` "/Game/InfiniteMatrix/Blueprints/BP_Tunnel.BP_Tunnel_C"))
      (for _array_element _outactors
        (`self.K2_DestroyActor` _array_element)
        (bind _outactors_2 (`GameplayStatics.GetAllActorsOfClass` "/Game/InfiniteMatrix/Blueprints/SM_Enemy.SM_Enemy_C" :!label _label))
        (for _array_element_2 _outactors_2
          (`self.K2_DestroyActor` _array_element_2))))
    (:`then_1`
      (for _ (range 3)
        (`/Engine/EditorBlueprintResources/StandardMacros.IsValid` (`self.Newest Tunnel`)
          (:`Is Valid`
            (`self.SpawnTunnelAtSpawnPoint`)
            (goto _label))
          (:`Is Not Valid`
            (`self.Spawn Tunnel` (`self.K2_GetActorLocation` (`GameplayStatics.GetPlayerPawn` 0)))
            (goto _label)))))))

(fn `SpawnTunnelAtSpawnPoint`
  (`self.Spawn Tunnel` (`SceneComponent.K2_GetComponentLocation` (`/Game/InfiniteMatrix/Blueprints/BP_Tunnel.SpawnPoint` (`self.Newest Tunnel`)))))

(fn `UserConstructionScript`)